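; GameCharacter is a player character Blueprint with mouse look, axis-driven movement and a gun attached as a child actor.
; Input axes move it along the capsule's forward and right vectors, while scaled mouse axes drive controller yaw and pitch.
; BeginPlay adds the HUD widget and passes the camera to the BaseGun child actor.
; The Fire action calls FireGun on that gun, printing an error if the BaseGun cast fails.
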(event EventBeginPlay
  (bind _returnvalue (UserInterface|CreateWidget "/Game/Blueprints/HUD.HUD_C"))
  (UserInterface|Viewport|AddtoViewport _returnvalue 0)
  (bind _asbase_gun (Utilities|Casting|CastToBaseGun (Variables|/Script/Engine.ChildActorComponent|GetChildActor (Variables|Default|GetGunActor))))
  (Class|BaseGun|SetCamera _asbase_gun (Variables|Default|GetCamera)))

(event Input|ActionEvents|InputActionFire
  (params (Key :type Key%20Structure))
  (:Pressed
    (bind _asbase_gun (Utilities|Casting|CastToBaseGun (Variables|/Script/Engine.ChildActorComponent|GetChildActor (Variables|Default|GetGunActor)))
      (:then
        (Class|BaseGun|FireGun _asbase_gun))
      (:CastFailed
        (Development|PrintString "Attacht Gun is not of BaseClass BaseGun" true false)))))

(event Input|AxisEvents|InputAxisHorizontal
  (params (AxisValue :type Float%20%28single-precision%29))
  (Pawn|Input|AddMovementInput (Math|Vector|GetRightVector (Variables|Default|GetCapsuleComponent)) AxisValue false))

(event Input|AxisEvents|InputAxisVertical
  (params (AxisValue :type Float%20%28single-precision%29))
  (Pawn|Input|AddMovementInput (Math|Vector|GetForwardVector (Variables|Default|GetCapsuleComponent)) AxisValue false))

(event Input|MouseEvents|MouseX
  (params (AxisValue :type Float%20%28single-precision%29))
  (Pawn|Input|AddControllerYawInput (* AxisValue 2.0)))

(event Input|MouseEvents|MouseY
  (params (AxisValue :type Float%20%28single-precision%29))
  (Pawn|Input|AddControllerPitchInput (* AxisValue -2.0)))

(fn ConstructionScript)